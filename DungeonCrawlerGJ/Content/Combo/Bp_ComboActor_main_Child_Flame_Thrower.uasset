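; Flame thrower variant of the main combo actor, a one-shot animated effect that removes itself when done.
; PlayAnim activates the Niagara effect and plays a timeline that slides the half-scale static mesh along local X, with the travel clamped, while a second track drives its yaw.
; The actor destroys itself when the timeline finishes, and construction defers to the parent.
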(event `self.PlayAnim`
  (`ActorComponent.Activate` (`self.Niagara`) false)
  (bind (_direction _newtrack_0 _newtrack_1) (`Timeline|Timeline_0` :!via `PlayFromStart`)
    (:`Update`
      (`SceneComponent.K2_SetRelativeTransform` (`self.StaticMesh`) (`KismetMathLibrary.MakeTransform` (`KismetMathLibrary.MakeVector` (+ (`KismetMathLibrary.FClamp` (* 500 _newtrack_0) 0.0 232.0) -200.0) 0.0 -20.0) (`KismetMathLibrary.MakeRotator` 0.0 0.0 _newtrack_1) (0.5 0.5 0.5)) false false))
    (:`Finished`
      (`self.K2_DestroyActor`))))

(fn `UserConstructionScript`
  (`parent.UserConstructionScript`))